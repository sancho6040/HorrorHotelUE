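; BP_PickUP is a pickup item actor whose ItemIndex selects its static mesh in the construction script.
; A box overlap with BP_MultiPlayerCharacter shows or hides a Plane VFX, which starts hidden.
; ItemPickedUpEvent prints a debug string, adds ItemIndex to the first top-level WB_InventoryUI widget found, then destroys the actor.
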(event `self.ItemPickedUpEvent`
  ;[1 0.3871 0.8383] PickedUp Event
  (`KismetSystemLibrary.PrintString` "Hello")
  (bind _foundwidgets (`WidgetBlueprintLibrary.GetAllWidgetsOfClass` "/Game/HorrorHotel_UE/Blueprints/UI/InGame/Inventory/WB_InventoryUI.WB_InventoryUI_C"))
  (`/Game/HorrorHotel_UE/Blueprints/UI/InGame/Inventory/WB_InventoryUI.AddItem` (`|GetArrayItem` _foundwidgets) (`self.ItemIndex`))
  (`self.K2_DestroyActor`))

(event `self.ReceiveBeginPlay`
  ;[0.1673 1 0.5197] VFX Visibility
  (`self.ToggleVFX` false))

(event `self.Box.OnComponentBeginOverlap`
  (params (OverlappedComponent :type "PrimitiveComponent Object Reference") (OtherActor :type "Actor Object Reference") (OtherComp :type "PrimitiveComponent Object Reference") (OtherBodyIndex :type Integer) (bFromSweep :type Boolean) (SweepResult :type "HitResult Structure (by ref)"))
  ;[0.1673 1 0.5197] VFX Visibility
  (cast `/Game/HorrorHotel_UE/Blueprints/Player/BP_MultiPlayerCharacter` OtherActor)
  (`self.ToggleVFX` true))

(event `self.Box.OnComponentEndOverlap`
  (params (OverlappedComponent :type "PrimitiveComponent Object Reference") (OtherActor :type "Actor Object Reference") (OtherComp :type "PrimitiveComponent Object Reference") (OtherBodyIndex :type Integer))
  ;[0.1673 1 0.5197] VFX Visibility
  (cast `/Game/HorrorHotel_UE/Blueprints/Player/BP_MultiPlayerCharacter` OtherActor)
  (`self.ToggleVFX` false))

(fn `ToggleVFX`
  (params (bNewVisibility :type Boolean))
  (`SceneComponent.SetVisibility` (`self.Plane`) bNewVisibility true))

(fn `UserConstructionScript`
  (`StaticMeshComponent.SetStaticMesh` (`self.StaticMesh`) (`|GetArrayItem` (`self.Meshes`) (`self.ItemIndex`))))